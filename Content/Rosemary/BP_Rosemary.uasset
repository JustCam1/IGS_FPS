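; Rosemary is an AI character that follows the player and whose death opens the game-over level.
; Perception updates start a self-repeating half-second loop that re-issues AIMoveTo toward the player controller.
; Damage drains Health, which Tick shows on a camera-facing widget bar, until a one-time death destroys the actor.
; Helper functions supply attack and defend ranges, a patrol route and walk speeds by movement state.
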(event OnPerceptionUpdated(AIPerception)
  (params (UpdatedActors :type Array%20of%20Actor%20Object%20References))
  (CallFunction|FollowPlayer))

(event Custom|FollowPlayer
  (Utilities|FlowControl|Delay 0.5)
  (AI|AIMoveTo self "0, 0, 0" (Game|GetPlayerController 0) 1e+01 true
    (:then
      (CallFunction|FollowPlayer))))

(event EventBeginPlay)

(event Game|Damage|EventAnyDamage
  (params (Damage :type Float%20%28single-precision%29) (DamageType :type Damage%20Type%20Object%20Reference) (InstigatedBy :type Controller%20Object%20Reference) (DamageCauser :type Actor%20Object%20Reference))
  (bind _output_get (Variables|Default|SetHealth (- (Variables|Default|GetHealth) Damage)))
  (if (<= _output_get 0.0)
    (Utilities|FlowControl|DoOnce false
      (:Completed
        (Variables|Default|SetisDead true)
        (Components|Movement|StopMovementImmediately (Variables|Character|GetCharacterMovement))
        (Actor|DestroyActor)
        (Game|OpenLevel(byObjectReference) "/Game/Levels/GameOverScreen.GameOverScreen")))))

(event EventTick
  (params (DeltaSeconds :type Float%20%28single-precision%29))
  (bind _healthbarrosemary (Variables|Default|GethealthBarRosemary))
  (bind _asrosemary_health (Utilities|Casting|CastToRosemaryHealth (UserInterface|GetWidget (Variables|Default|GethealthBarRosemary))))
  (Progress|SetPercent (Variables|/Game/Alex/AlexM/UI/RosemaryHealth.RosemaryHealth_C|GethealthBarRosemary _asrosemary_health) (/ (Variables|Default|GetHealth) 1e+02))
  (Transformation|SetWorldRotation _healthbarrosemary (Math|Rotator|FindLookatRotation (Transformation|GetWorldLocation _healthbarrosemary) (Transformation|GetWorldLocation (Variables|/Script/Engine.PlayerCameraManager|GetTransformComponent (Game|GetPlayerCameraManager 0)))) false false))

(fn ConstructionScript)

(fn GetIdealRange
  (return 1.5e+02 3.5e+02))

(fn GetPatrolRoute
  (return (Variables|AI|GetPatrolRoutes)))

(fn SetMovementSpeed
  (params (Speed :type E_MovementSpeed%20Enum :default "NewEnumerator0"))
  (bind _output_get (Variables|/Script/Engine.CharacterMovementComponent|SetMaxWalkSpeed (Variables|Character|GetCharacterMovement) (Utilities|Select :Index Speed :NewEnumerator0 0.0 :NewEnumerator1 5e+01 :NewEnumerator2 1e+02 :NewEnumerator3 2e+02)))
  (return _output_get))