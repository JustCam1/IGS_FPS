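; Base zombie enemy character that chases and attacks the player until damage kills it.
; ChasePlayer issues AIMoveTo, attacks without waiting for arrival and repeats after a delay; nothing in this graph starts it.
; Attack plays a montage and fires AttackOnEnd; lethal damage plays a death montage, then destroys the actor after delays.
; GetPatrolRoute exposes patrol routes, while SetMovementSpeed is a stub returning zero.
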(event Custom|ChasePlayer
  (if (not (Variables|Default|GetisDead))
    (AI|AIMoveTo self "0, 0, 0" (Game|GetPlayerCharacter 0) 5e+01 false
      (:then
        (CallFunction|Attack)
        (Utilities|FlowControl|Delay 3.0)
        (CallFunction|ChasePlayer)))))

(event Custom|Attack
  (if (not (Variables|Default|GetisDead))
    (Animation|Montage|PlayMontage (Variables|Character|GetMesh) "/Game/ZombieAnimations/Scratch_Zombie__female/Zombie_Attack_Montage.Zombie_Attack_Montage"
      (:OnCompleted
        _)
      (:OnInterrupted
        _))
    (Default|CallAttackonEnd)))

(event EventBeginPlay)

(event Game|Damage|EventAnyDamage
  (params (Damage :type Float%20%28single-precision%29) (DamageType :type Damage%20Type%20Object%20Reference) (InstigatedBy :type Controller%20Object%20Reference) (DamageCauser :type Actor%20Object%20Reference))
  (bind _output_get (Variables|Default|SetHealth (- (Variables|Default|GetHealth) Damage)))
  (if (<= _output_get 0.0)
    (Utilities|FlowControl|DoOnce false
      (:Completed
        (Variables|Default|SetisDead true)
        (Animation|Montage|PlayMontage (Variables|Character|GetMesh) "/Game/ZombieAnimations/Scratch_Zombie__female/Zombie_Dying_Montage.Zombie_Dying_Montage"
          (:then
            _)
          (:OnCompleted
            _))
        (Utilities|FlowControl|Delay 5.0)
        (Utilities|FlowControl|Delay 3.0)
        (Actor|DestroyActor)
        (Collision|SetCollisionEnabled (Variables|Collision|GetCapsuleComponent) "NoCollision")))))

(fn ConstructionScript)

(fn GetPatrolRoute
  (return (Variables|AI|GetPatrolRoutes)))

(fn SetMovementSpeed
  (params (Speed :type E_MovementSpeed%20Enum :default "NewEnumerator0"))
  (return 0.0))