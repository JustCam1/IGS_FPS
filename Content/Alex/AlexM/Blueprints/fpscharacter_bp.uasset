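; First-person player character for a zombie game, handling movement, flashlight, pause, health with hit feedback, and game over.
; A child actor holds the current weapon (none, pistol or machete), re-cast and socketed to the hands on swaps, with ammo and durability kept in structs.
; Montages drive reload and swing, with sphere-traced blade hits.
; Tick line-traces tagged interactables for a prompt and rotates the pistol arms near walls.
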(event Custom|Update
  ;[1 1 1] This is so we can reference the BaseWeapon_BP
  (bind _asbase_weapon_bp (Utilities|Casting|CastToBaseWeapon_BP (Variables|/Script/Engine.ChildActorComponent|GetChildActor (Variables|Default|GetWeapon_Child_Actor))))
  (bind _output_get (Variables|Default|SetWeaponRef _asbase_weapon_bp))
  (Variables|/Game/Alex/AlexM/Blueprints/Alex_Weapons/BaseWeapon_BP.BaseWeapon_BP_C|SetPlayerRef _output_get self)
  ;[1 1 1] Sets the Crosshair
  (bind _returnvalue (UserInterface|CreateWidget "/Game/Alex/AlexM/UI/Playerhud_BP.Playerhud_BP_C"))
  (bind _output_get_2 (Variables|Default|SetplayerHudRef _returnvalue))
  (UserInterface|Viewport|AddtoViewport _output_get_2 0)
  (CallFunction|AttachWeapontoHands) ; Calls the function
  (Variables|Default|SetCanAttack true) ; Can Attack is set to true by default
)

(event Custom|Melee%20Damage%20DelayTaken
  ;[1 1 1] Melee Damage Delay Taken - This is called from our FPSHit Detect function so the melee weapon can take damage.
  (if (Variables|Default|GetEnemyIsHit)
    (Default|MeleeDamageTaken (Variables|Default|GetWeaponRef))
    (Utilities|FlowControl|Delay 1.0)
    (Variables|Default|SetEnemyIsHit false) ; This is to allow our machete to detect\nagain.
  ))

(event Custom|RayTrace
  (bind _camera (Variables|Default|GetCamera))
  (bind _returnvalue (Transformation|GetWorldLocation _camera))
  ;[1 1 1] RayTrace - This is our RayTrace or Raycast Function.
  (bind _outhit (Collision|LineTraceByChannel _returnvalue (+ _returnvalue (* (Math|Vector|GetForwardVector _camera) (Variables|Default|GetInteraction_Distance))) "TraceTypeQuery1" false 0 "None"))
  (if (and (.bBlockingHit (Collision|BreakHitResult _outhit)) (Utilities|DoesObjectImplementInterface (.HitActor (Collision|BreakHitResult _outhit)) "/Game/Alex/AlexM/Blueprints/Interaction_Interface.Interaction_Interface_C"))
    (Variables|Default|SetTarget_Interface (.HitActor (Collision|BreakHitResult _outhit)))
    (Variables|Default|SetHit%20Component (.HitComponent (Collision|BreakHitResult _outhit)))
    (Variables|Default|SetCastingIsTrue true)
    (CallFunction|CheckTags)
    (else
      (Variables|Default|SetTarget_Interface 0)
      (Variables|Default|SetHit%20Component 0)
      (Variables|Default|SetCastingIsTrue false)
      (CallFunction|RemovefromVP))))

(event Custom|UpdatePlayerMovement
  (bind _returnvalue (Transformation|GetActorRotation))
  (bind _charactermovement (Variables|Character|GetCharacterMovement))
  ;[1 1 1] Update Player Movement - This updates our players movement as collisions collides with our character
  (Class|MovementComponent|MoveUpdatedComponent _charactermovement "0.100000,0.100000,0.000000" _returnvalue true)
  (Class|MovementComponent|MoveUpdatedComponent _charactermovement "-0.100000,-0.100000,0.000000" _returnvalue true))

(event Custom|Pistol_BP_Reference
  (bind _weapon_child_actor (Variables|Default|GetWeapon_Child_Actor))
  (bind _childactor (Variables|/Script/Engine.ChildActorComponent|GetChildActor _weapon_child_actor))
  ;[1 1 1] Pistol Cast - Casting into the Pistol.
  (if (== (.weapon (Variables|Default|GetPistol)) _childactor) ; if our child actor component\nis equal to the Pistol Weapon\nClass, then we cast.
    (bind _aspistol_bp (Utilities|Casting|CastToPistol_BP _childactor)) ; This is casted to the Pistol BP referenced\nfrom the child actor. This allows us to reference\nthe variables within that BP.
    (Variables|Default|SetPistol_BP_Var _aspistol_bp) ; Basically setting a Constructor\nfrom that BP
  ))

(event Custom|Ammo_Holder
  (bind _weaponref (Variables|Default|GetWeaponRef))
  ;[1 1 1] Ammo Holder - This sets and holds our ammo count for the Pistol.
  (Variables|Default|SetPistol (Utilities|Struct|MakeWeaponStruct (.weapon (Variables|Default|GetPistol)) (Variables|/Game/Alex/AlexM/Blueprints/Alex_Weapons/BaseWeapon_BP.BaseWeapon_BP_C|GetCurrent%20Ammo _weaponref) (Variables|/Game/Alex/AlexM/Blueprints/Alex_Weapons/BaseWeapon_BP.BaseWeapon_BP_C|GetMax%20Ammo _weaponref) 0.0 0.0)) ; This sets the Pistol Weapon Struct\nto hold the current Ammo and\ncurrent Max Ammo
)

(event Custom|AttachWeaponToHands
  (bind _weaponref (Variables|Default|GetWeaponRef))
  (bind _playerhudref (Variables|Default|GetplayerHudRef))
  ;[1 1 1] Animation Player - Sets our fps character to whichever animation and widget screen based upon the Weapon Blueprint that has been casted to from the Update Function and attaches the weapon or non-weapon onto the player.
  (Transformation|AttachComponentToComponent (Variables|/Game/Alex/AlexM/Blueprints/Alex_Weapons/BaseWeapon_BP.BaseWeapon_BP_C|GetWeapon _weaponref) (Variables|Default|GetFPSHands) (Variables|/Game/Alex/AlexM/Blueprints/Alex_Weapons/BaseWeapon_BP.BaseWeapon_BP_C|GetSocket _weaponref) "SnapToTarget" "SnapToTarget" "SnapToTarget" true)
  (Variables|Default|SetAnim (Variables|/Game/Alex/AlexM/Blueprints/Alex_Weapons/BaseWeapon_BP.BaseWeapon_BP_C|GetAnimation _weaponref))
  (Variables|Default|SetWeaponTarget (Variables|/Game/Alex/AlexM/Blueprints/Alex_Weapons/BaseWeapon_BP.BaseWeapon_BP_C|GetWeaponName _weaponref))
  (switch string (Utilities|String|ToString(Text) (Variables|Default|GetWeaponTarget))
    (:Pistol
      (Default|GunStatus _playerhudref)
      (Variables|Default|SetNoWeaponPose false))
    (:Machete
      (Default|MeleeStatus _playerhudref)
      (Variables|Default|SetNoWeaponPose false))
    (:No%20Weapon
      (Default|NoStatus _playerhudref)
      (Variables|Default|SetNoWeaponPose true))))

(event Custom|Check%20Tags
  (bind _hit_component (Variables|Default|GetHit%20Component))
  ;[1 1 1] Check Tags - This checks the tag of any objects, whether is interactable or not.
  (bind _output_get (Variables|/Script/Engine.ActorComponent|SetComponentTags _hit_component (Variables|/Script/Engine.ActorComponent|GetComponentTags _hit_component)))
  (bind _output_get_2 (Variables|Default|SetTag_Names _output_get))
  (for _array_element _output_get_2
    (switch string (Utilities|String|ToString(Name) _array_element)
      (:Default
        (CallFunction|RemovefromVP :!label _label)
        (Variables|Default|SetNameDetected ""))
      (:Handle
        (CallFunction|AddtoVP :!label _label_2)
        (Variables|Default|SetNameDetected (Utilities|String|StringToName (Utilities|String|ToString(Name) _array_element))))
      (:Interactive
        (goto _label_2))
      (:Door
        (goto _label_2))
      (:None
        (goto _label))
      (:Null
        (goto _label))
      (:Medkit
        (goto _label_2))
      (:Gun
        (goto _label_2))
      (:Melee
        (goto _label_2))
      (:Lever
        (goto _label_2)))))

(event Custom|UnlockDoor
  ;[1 1 1] UnlocksDoorForArmory
  (Utilities|FlowControl|DoOnce false
    (:Completed
      (bind _returnvalue (Actor|GetActorOfClass "/Game/cam/Door/Door.Door_C"))
      (Default|UnlockDoor _returnvalue)
      (Development|PrintString "Working in fps")
      (Audio|PlaySound2D "/Game/SoundsNMusic/IGSMusicSoundsSomething/DoorUnlock.DoorUnlock" 1.0 1.0 0.0 0 0))))

(event Custom|AddToVP
  ;[1 1 1] Adding and Removing View Ports Functions
  (if (not (Variables|Default|GetEPressed))
    (UserInterface|Viewport|AddtoViewport (Variables|Default|GetInteractive%20UI%20Ref) 0)))

(event Custom|RemoveFromVP
  ;[1 1 1] Adding and Removing View Ports Functions
  (Widget|RemovefromParent (Variables|Default|GetInteractive%20UI%20Ref)))

(event Custom|Weapon_Pose
  (bind _pistol_bp_var (Variables|Default|GetPistol_BP_Var))
  (bind _fpshands (Variables|Default|GetFPSHands))
  ;[1 1 1] Weapon Pose - This rotates the pistol if it hits a wall or collision.
  (Variables|Default|SetMoveArm (Variables|/Game/Alex/AlexM/Blueprints/Alex_Weapons/Pistol_BP.Pistol_BP_C|GetWall_Hit _pistol_bp_var))
  (Variables|Default|SetMoveArm2 (Variables|/Game/Alex/AlexM/Blueprints/Alex_Weapons/Pistol_BP.Pistol_BP_C|GetOuter_Trace _pistol_bp_var))
  (if (Variables|Default|GetMoveArm)
    (Transformation|AddRelativeRotation _fpshands "0.000000,0.000000,5.000000" false false)
    (Variables|Default|SetPistol_Pose_On? true)
    (elif (not (Variables|Default|GetMoveArm2))
      (Transformation|SetRelativeRotation _fpshands (Math|Interpolation|RInterpTo (Variables|/Script/Engine.SceneComponent|GetRelativeRotation _fpshands) "0.000000,-90.000000,80.000000" (Utilities|Time|GetWorldDeltaSeconds) 5.0) false false)
      (if (<= (.roll (Variables|/Script/Engine.SceneComponent|GetRelativeRotation (Variables|Default|GetFPSHands))) 85.0)
        (Variables|Default|SetPistol_Pose_On? false)))))

(event Input|EnhancedActionEvents|EnhancedInputActionMove_IA
  (params (ActionValue :type Vector%202D%20Structure) (ElapsedSeconds :type Float%20%28double-precision%29) (TriggeredSeconds :type Float%20%28double-precision%29) (InputAction :type Input%20Action%20Object%20Reference :default "/Game/Alex/AlexM/Input/Move_IA.Move_IA"))
  ;[1 1 1] Handle Movement
  (Pawn|Input|AddMovementInput (Transformation|GetActorRightVector) (.x ActionValue) false) ; This allows us to move our player. It\ntakes in 2 values, world direction and\nscale values.\nWorld Direction tells us where are player\nin the game should move.\nThe Scale Value will tell us if we should\nmove positvely or negatively in this \ndirection.
  (Pawn|Input|AddMovementInput (Transformation|GetActorForwardVector) (.y ActionValue) false))

(event Input|EnhancedActionEvents|EnhancedInputActionLook_IA
  (params (ActionValue :type Vector%202D%20Structure) (ElapsedSeconds :type Float%20%28double-precision%29) (TriggeredSeconds :type Float%20%28double-precision%29) (InputAction :type Input%20Action%20Object%20Reference :default "/Game/Alex/AlexM/Input/Look_IA.Look_IA"))
  ;[1 1 1] Handle Camera Movement
  (Pawn|Input|AddControllerYawInput (.x ActionValue))
  (Pawn|Input|AddControllerPitchInput (.y ActionValue)))

(event Input|EnhancedActionEvents|EnhancedInputActionSwap_Melee_IA
  (params (ActionValue :type Boolean) (ElapsedSeconds :type Float%20%28double-precision%29) (TriggeredSeconds :type Float%20%28double-precision%29) (InputAction :type Input%20Action%20Object%20Reference :default "/Game/Alex/AlexM/Input/Swap_Melee_IA.Swap_Melee_IA"))
  (bind _weaponref (Variables|Default|GetWeaponRef))
  (bind _machete (Variables|Default|GetMachete))
  ;[1 1 1] Swap_Melee_IA - Swaps to Melee Logic
  (:Started
    (if (Variables|Default|GetHas_Melee) ; Checks condition if Has\nMelee is true.
      (switch string (Utilities|String|ToString(Text) (Variables|Default|GetWeaponTarget)) ; If player is in No Weapon or Pistol Mode.
        (:No%20Weapon
          _)
        (:Pistol
          _))
      (if (and (not (Variables|Default|GetIsReloading)) (not (Variables|Default|GetPistol_Pose_On?))) ; If player is not reloading and\ngun rotation is not down.
        (CallFunction|AmmoHolder) ; Calls the Ammo Holder Function
        (ChildActorComponent|SetChildActorClass (Variables|Default|GetWeapon_Child_Actor) (.weapon (Variables|Default|GetMachete))) ; Sets the child actor class of our fps \ncharacter to become the Machete Class
        (Widget|RemovefromParent (Variables|Default|GetplayerHudRef)) ; Then we'll remove whatever what on\nthe hud
        (CallFunction|Update) ; We'll play the Update Function.
        ;[1 1 1] Machete Set Up
        (Variables|/Game/Alex/AlexM/Blueprints/Alex_Weapons/BaseWeapon_BP.BaseWeapon_BP_C|SetMeleeHealth _weaponref (.meleehealth _machete)) ; We'll set the Machete Weapon Struct to become whatever\nthe Melee Health and Max Health is so the machete will have\nthese features when played upon.
        (Variables|/Game/Alex/AlexM/Blueprints/Alex_Weapons/BaseWeapon_BP.BaseWeapon_BP_C|SetMeleeMaxHealth _weaponref (.meleemaxhealth _machete))
        (Variables|Default|SetMacheteEquipped true) ; Machete is now Equipped.
      ))))

(event Input|EnhancedActionEvents|EnhancedInputActionSwap_Gun_IA
  (params (ActionValue :type Boolean) (ElapsedSeconds :type Float%20%28double-precision%29) (TriggeredSeconds :type Float%20%28double-precision%29) (InputAction :type Input%20Action%20Object%20Reference :default "/Game/Alex/AlexM/Input/Swap_Gun_IA.Swap_Gun_IA"))
  (bind _weaponref (Variables|Default|GetWeaponRef))
  (bind _weaponref_2 (Variables|Default|GetWeaponRef))
  (bind _pistol (Variables|Default|GetPistol))
  ;[1 1 1] Swap_Pistol_IA - This swaps to the pistol when the player presses 2.
  (:Started
    (switch string (Utilities|String|ToString(Text) (Variables|Default|GetWeaponTarget)) ; This checks if the player is in no weapon\nor machete position, if the character is,\nthen continue to the branch
      (:No%20Weapon
        _)
      (:Machete
        _))
    (if (and (not (Variables|Default|GetSwing)) (not (Variables|Default|GetPistol_Pose_On?)))
      (Variables|Default|SetMachete (Utilities|Struct|MakeWeaponStruct (.weapon (Variables|Default|GetMachete)) 0 0 (Variables|/Game/Alex/AlexM/Blueprints/Alex_Weapons/BaseWeapon_BP.BaseWeapon_BP_C|GetMeleeHealth _weaponref) (Variables|/Game/Alex/AlexM/Blueprints/Alex_Weapons/BaseWeapon_BP.BaseWeapon_BP_C|GetMeleeMaxHealth _weaponref))) ; This sets and hold the values of our Machete
      (ChildActorComponent|SetChildActorClass (Variables|Default|GetWeapon_Child_Actor) (.weapon (Variables|Default|GetPistol))) ; Sets Child Actor Class to Weapon
      (Widget|RemovefromParent (Variables|Default|GetplayerHudRef))
      (CallFunction|Update)
      (Variables|/Game/Alex/AlexM/Blueprints/Alex_Weapons/BaseWeapon_BP.BaseWeapon_BP_C|SetCurrent%20Ammo _weaponref_2 (.currentammo _pistol))
      (Variables|/Game/Alex/AlexM/Blueprints/Alex_Weapons/BaseWeapon_BP.BaseWeapon_BP_C|SetMax%20Ammo _weaponref_2 (.maxammo _pistol))
      (CallFunction|PistolBPReference) ; This is a function to cast into the\npistol Blueprint Class.
      (Variables|Default|SetMacheteEquipped false) ; Machete is not equipped now
    )))

(event Input|EnhancedActionEvents|EnhancedInputActionJump_IA
  (params (ActionValue :type Boolean) (ElapsedSeconds :type Float%20%28double-precision%29) (TriggeredSeconds :type Float%20%28double-precision%29) (InputAction :type Input%20Action%20Object%20Reference :default "/Game/Alex/AlexM/Input/Jump_IA.Jump_IA"))
  ;[1 1 1] Handle Jumping
  (:Started
    (Character|Jump))
  (:Completed
    (Character|StopJumping)))

(event Input|EnhancedActionEvents|EnhancedInputActionFlashLight_IA
  (params (ActionValue :type Boolean) (ElapsedSeconds :type Float%20%28double-precision%29) (TriggeredSeconds :type Float%20%28double-precision%29) (InputAction :type Input%20Action%20Object%20Reference :default "/Game/Alex/AlexM/Input/FlashLight_IA.FlashLight_IA"))
  ;[1 1 1] Flashlight Mechanics
  (:Started
    (Utilities|FlowControl|FlipFlop ; Toggles Flashlight
      (:A
        (Rendering|SetVisibility (Variables|Default|GetFlashlight) true false) ; Sets Flashlight On
      )
      (:B
        (Rendering|SetVisibility (Variables|Default|GetFlashlight) false false) ; Sets Flashlight Off
      ))))

(event Input|EnhancedActionEvents|EnhancedInputActionChangeMode_AI
  (params (ActionValue :type Boolean) (ElapsedSeconds :type Float%20%28double-precision%29) (TriggeredSeconds :type Float%20%28double-precision%29) (InputAction :type Input%20Action%20Object%20Reference :default "/Game/Alex/AlexM/Input/ChangeMode_AI.ChangeMode_AI")))

(event Input|EnhancedActionEvents|EnhancedInputActiontestDamge
  (params (ActionValue :type Boolean) (ElapsedSeconds :type Float%20%28double-precision%29) (TriggeredSeconds :type Float%20%28double-precision%29) (InputAction :type Input%20Action%20Object%20Reference :default "/Game/Alex/AlexM/Input/testDamge.testDamge"))
  (bind _returnvalue (Actor|GetActorOfClass "/Game/Enemy_Base/GirlZombie/BP_EnemyBase.BP_EnemyBase_C"))
  (Class|AISenseDamage|ReportDamageEvent _returnvalue self 1e+01 (Transformation|GetActorLocation) "0, 0, 0" "None"))

(event Input|EnhancedActionEvents|EnhancedInputActionPauseMenu_IA
  (params (ActionValue :type Boolean) (ElapsedSeconds :type Float%20%28double-precision%29) (TriggeredSeconds :type Float%20%28double-precision%29) (InputAction :type Input%20Action%20Object%20Reference :default "/Game/Alex/AlexM/Input/PauseMenu_IA.PauseMenu_IA"))
  (bind _returnvalue (Game|GetPlayerController 0))
  (bind _returnvalue_2 (UserInterface|CreateWidget "/Game/Nikolas/Pausemenu_WB.Pausemenu_WB_C"))
  (UserInterface|Viewport|AddtoViewport _returnvalue_2 0)
  (Variables|/Script/Engine.PlayerController|SetbShowMouseCursor _returnvalue true)
  (Input|SetInputModeUIOnly _returnvalue 0 "DoNotLock" false)
  (Game|SetGamePaused true))

(event Input|EnhancedActionEvents|EnhancedInputActionInteract_IA
  (params (ActionValue :type Boolean) (ElapsedSeconds :type Float%20%28double-precision%29) (TriggeredSeconds :type Float%20%28double-precision%29) (InputAction :type Input%20Action%20Object%20Reference :default "/Game/Alex/AlexM/Input/Interact_IA.Interact_IA"))
  (bind _interactive_ui_ref (Variables|Default|GetInteractive%20UI%20Ref))
  ;[1 1 1] Interact_IA - This is so we can press E on interactive Assets.
  (:Started
    (if (Variables|Default|GetCastingIsTrue)
      (for _array_element (Variables|Default|GetTag_Names)
        (switch string (Utilities|String|ToString(Name) _array_element)
          (:Handle
            (if (not (Variables|Default|GetEPressed)) :!label _label
              (Variables|Default|SetEPressed true)
              (Class|InteractionInterface|Interact(Message) (Variables|Default|GetTarget_Interface))
              (CallFunction|RemovefromVP)
              (Utilities|FlowControl|Delay 0.5)
              (Variables|Default|SetEPressed false)))
          (:Interactive
            (goto _label))
          (:Door
            (goto _label))
          (:Medkit
            (if (< (Variables|Default|Gethealth) 1e+02)
              (goto _label)
              (else
                (Default|MaxHealth _interactive_ui_ref)
                (Utilities|FlowControl|Delay 0.5)
                (Default|Press[E] _interactive_ui_ref))))
          (:Gun
            (goto _label))
          (:Melee
            (goto _label))
          (:Lever
            (goto _label)))))))

(event Input|EnhancedActionEvents|EnhancedInputActionAttack_IA
  (params (ActionValue :type Boolean) (ElapsedSeconds :type Float%20%28double-precision%29) (TriggeredSeconds :type Float%20%28double-precision%29) (InputAction :type Input%20Action%20Object%20Reference :default "/Game/Alex/AlexM/Input/Attack_IA.Attack_IA"))
  (bind _weaponref (Variables|Default|GetWeaponRef))
  ;[1 1 1] Attack IA - This is where the character of our player attacks when the RMB is clicked.
  (:Started
    (Utilities|IsValid (Variables|Default|GetWeaponRef)
      (:Is%20Valid
        (if (Math|Boolean|ANDBoolean (not (Variables|Default|GetIsReloading)) (not (Variables|Default|GetPistol_Pose_On?)) (not (Variables|Default|GetNoWeaponPose)) (Variables|Default|GetCanAttack))
          (Variables|Default|SetAttack true) ; Sets Attacking State on
          (Variables|Default|SetCanAttack false) ; Sets Can Attack to false, because\nwe are attacking at this point.
          (switch string (Utilities|String|ToString(Text) (Variables|Default|GetWeaponTarget)) ; Switch-Case, Checks for whichever\nweapon we are holding at hand
            (:Pistol
              (Default|StartShooting (Variables|Default|GetWeaponRef)) ; This references the Start Shooting Function\nfrom the Base Weapon BP.
              (bind _returnvalue (Actor|GetActorOfClass "/Game/Enemy_Base/AIFunctions/AIC_EnemyBase.AIC_EnemyBase_C")) ; This gets the class of the AI Zombie, so we can\ndo hit mechanics with this.
              (Class|AISenseDamage|ReportDamageEvent _returnvalue self 1e+01 (Transformation|GetActorLocation) "0, 0, 0" "None") ; This is how much damage we deal\nto the AI Zombie with the gun.
              (Utilities|FlowControl|Delay 0.51) ; Delay Timer
              (Variables|Default|SetAttack false) ; Set Attack to False
              (Variables|Default|SetCanAttack true) ; Set Can Attack to true.
              (if (and (> (Variables|/Game/Alex/AlexM/Blueprints/Alex_Weapons/BaseWeapon_BP.BaseWeapon_BP_C|GetMax%20Ammo _weaponref) 0) (< (Variables|/Game/Alex/AlexM/Blueprints/Alex_Weapons/BaseWeapon_BP.BaseWeapon_BP_C|GetCurrent%20Ammo _weaponref) (Variables|/Game/Alex/AlexM/Blueprints/Alex_Weapons/BaseWeapon_BP.BaseWeapon_BP_C|GetMag _weaponref))) ; If this is all true, then the gun can still reload.\nIf false, then the gun can not reload.
                (Variables|Default|SetCanReload true) ; Sets reload to True
                (else
                  (Variables|Default|SetCanReload false) ; Sets reload to False
                ))
              (if (<= (Variables|/Game/Alex/AlexM/Blueprints/Alex_Weapons/BaseWeapon_BP.BaseWeapon_BP_C|GetCurrent%20Ammo (Variables|Default|GetWeaponRef)) 0) ; Checks if the ammo is less than 0,\nif it is then play the sound effect.
                (Audio|PlaySound2D "/Game/Alex/AlexM/Sound_Effects/Sound_Effect_-_Gun_Dry_Firing.Sound_Effect_-_Gun_Dry_Firing" 1.0 1.0 0.0 0 0) ; Sound of effect of no more bullets when shooting,
              ))
            (:Machete
              (Variables|Default|SetSwing true) ; This is to differentiate the swing\nof the melee weapon, in this case,\nMachete
              (Animation|Montage|PlayMontage (Variables|Default|GetFPSHands) "/Game/Alex/AlexM/Blender_FPS/Machete/NewMacheteSing_Montage.NewMacheteSing_Montage" ; Plays the animation of the player swinging.
                (:then
                  (Utilities|FlowControl|Delay 1.85) ; Delay Timer
                  (Variables|Default|SetSwing false) ; Set Swing to false
                  (Variables|Default|SetAttack false) ; Set Attack to false
                  (Variables|Default|SetCanAttack true) ; Set Attack to true now, because we \nare out of the attack animation
                )))))))))

(event Input|EnhancedActionEvents|EnhancedInputActionReload_IA
  (params (ActionValue :type Boolean) (ElapsedSeconds :type Float%20%28double-precision%29) (TriggeredSeconds :type Float%20%28double-precision%29) (InputAction :type Input%20Action%20Object%20Reference :default "/Game/Alex/AlexM/Input/Reload_IA.Reload_IA"))
  (bind _weaponref (Variables|Default|GetWeaponRef))
  ;[1 1 1] Reload IA - This is a logic to reload the pistol
  (:Started
    (if (Math|Boolean|ANDBoolean (Variables|Default|GetCanReload) (not (Variables|Default|GetPistol_Pose_On?)) (not (Variables|Default|GetMacheteEquipped)) (not (Variables|Default|GetNoWeaponPose)) (< (Variables|/Game/Alex/AlexM/Blueprints/Alex_Weapons/BaseWeapon_BP.BaseWeapon_BP_C|GetCurrent%20Ammo _weaponref) (Variables|/Game/Alex/AlexM/Blueprints/Alex_Weapons/BaseWeapon_BP.BaseWeapon_BP_C|GetMag _weaponref)))
      (Variables|Default|SetIsReloading true) ; If the condition passes, we set\nis reloading to true, because we \nare in this animation of reloading.
      (Variables|Default|SetCanReload false) ; Can Reload is set to false, because\nwe are already reloading.
      (switch string (Utilities|String|ToString(Text) (Variables|Default|GetWeaponTarget)) ; Checks what our Weapon Target is set to.
        (:Pistol
          (Animation|Montage|PlayMontage (Variables|Default|GetFPSHands) "/Game/Alex/AlexM/Blender_FPS/Pistol/Arms_Reload_Montage.Arms_Reload_Montage" ; Because our Weapon Target is Pistol, then we can play the\nFPS character reload animation.
            (:then
              (Components|Animation|PlayAnimation (Variables|/Game/Alex/AlexM/Blueprints/Alex_Weapons/BaseWeapon_BP.BaseWeapon_BP_C|GetWeapon (Variables|Default|GetWeaponRef)) "/Game/Alex/AlexM/Blender_FPS/Pistol/Pistol_Gun_Reload_Anim.Pistol_Gun_Reload_Anim" false) ; This animation is set for the skeletal mesh component\nof our weapon ref, which is the pistol. So this plays\nthe slider to move back on the pistol.
              (Audio|PlaySound2D "/Game/MilitaryWeapSilver/Sound/Pistol/Wavs/Pistol_ReloadMagEject01.Pistol_ReloadMagEject01" 1.0 1.0 0.0 0 0) ; Plays the sound of the pistol slide.
              (Utilities|FlowControl|Delay 1.3)
              (Audio|PlaySound2D "/Game/MilitaryWeapSilver/Sound/Pistol/Wavs/Pistol_ReloadMagInsert01.Pistol_ReloadMagInsert01" 1.0 1.0 0.0 0 0) ; Plays the sound of the Magazine \ninserted into the gun.
              (Utilities|FlowControl|Delay 1.0)
              (Default|Reload (Variables|Default|GetWeaponRef)) ; This is the logic function that we call upon\nto fill our magazine with the difference set\nfrom the Max Ammo and the Mag Size.
              (Variables|Default|SetIsReloading false) ; After animation of reloading\nis done, we can set is reloading\nto false now.
            )))))))

(event EventBeginPlay
  ;[1 1 1] Add Input Controllers
  (bind _asplayer_controller (Utilities|Casting|CastToPlayerController (Pawn|GetController))) ; As soon as the game starts, this function\nwill gather the Actor or Object component\nand the Player Controller Reference (which\nis the Enhanced Input Local Player \nSubsystem), then execute to continue to\nthe next functions.\n\nThis function is all about gathering information.
  (Utilities|IsValid (PlayerController|LocalPlayerSubsystems|GetEnhancedInputLocalPlayerSubsystem _asplayer_controller) ; Once Cast To PlayerController has been ran,\nit will run into this function to see if the \ninput object is valid. If it's valid, then it executes\nto the next function, if not it will stop.
    (:Is%20Valid
      (Input|AddMappingContext (PlayerController|LocalPlayerSubsystems|GetEnhancedInputLocalPlayerSubsystem _asplayer_controller) "/Game/Alex/AlexM/Input/fps_ioc.fps_ioc" 0 "(bIgnoreAllPressedKeysUntilRelease=True,bForceImmediately=False,bNotifyUserSettings=False)") ; Target -   This is the Player Controller Reference.\nMapping Context - This is the Mapping Context Reference.\nPriority - Higher priority mappings will be applied first and, \n                  if they consume input, will block lower priority \n                  mappings.\nOption -  Options to consider when adding this Mapping Context.
      (Variables|Default|SetFuse_Lever_Count 0) ; This sets the Fuse Lever Count to 0
      (bind _returnvalue (UserInterface|CreateWidget "/Game/Alex/AlexM/UI/PlayerHealthBar.PlayerHealthBar_C" (Game|GetPlayerController 0)))
      (UserInterface|Viewport|AddtoViewport _returnvalue 0)
      ;[1 1 1] Flash Light Mechanics
      (Rendering|SetVisibility (Variables|Default|GetFlashlight) false false) ; Sets the flashlight off by default
      (ChildActorComponent|SetChildActorClass (Variables|Default|GetWeapon_Child_Actor) (.weapon (Variables|Default|GetNoWeapon)))
      (bind _returnvalue_2 (UserInterface|CreateWidget "/Game/Alex/AlexM/UI/Interact_BP.Interact_BP_C"))
      (Variables|Default|SetInteractive%20UI%20Ref _returnvalue_2)
      ;[1 1 1] This is so we can reference the BaseWeapon_BP
      (bind _asbase_weapon_bp (Utilities|Casting|CastToBaseWeapon_BP (Variables|/Script/Engine.ChildActorComponent|GetChildActor (Variables|Default|GetWeapon_Child_Actor))))
      (bind _output_get (Variables|Default|SetWeaponRef _asbase_weapon_bp))
      (Variables|/Game/Alex/AlexM/Blueprints/Alex_Weapons/BaseWeapon_BP.BaseWeapon_BP_C|SetPlayerRef _output_get self)
      ;[1 1 1] Sets the Crosshair
      (bind _returnvalue_3 (UserInterface|CreateWidget "/Game/Alex/AlexM/UI/Playerhud_BP.Playerhud_BP_C"))
      (bind _output_get_2 (Variables|Default|SetplayerHudRef _returnvalue_3))
      (UserInterface|Viewport|AddtoViewport _output_get_2 0)
      (CallFunction|AttachWeapontoHands) ; Calls the function
      (Variables|Default|SetCanAttack true) ; Can Attack is set to true by default
    )))

(event Collision|EventActorBeginOverlap
  (params (OtherActor :type Actor%20Object%20Reference)))

(event EventTick
  (params (DeltaSeconds :type Float%20%28single-precision%29))
  ;[1 1 1] Event Tick - Calls upon these function ever frame.
  (CallFunction|UpdatePlayerMovement)
  (CallFunction|RayTrace)
  (if (== (.weapon (Variables|Default|GetPistol)) (Variables|/Script/Engine.ChildActorComponent|GetChildActor (Variables|Default|GetWeapon_Child_Actor)))
    (CallFunction|WeaponPose)))

(event Game|Damage|EventAnyDamage
  (params (Damage :type Float%20%28single-precision%29) (DamageType :type Damage%20Type%20Object%20Reference) (InstigatedBy :type Controller%20Object%20Reference) (DamageCauser :type Actor%20Object%20Reference))
  ;[1 1 1] Event Any Damage - This function is when the player Takes in Any Damage from AI.
  (Variables|Default|Sethealth (- (Variables|Default|Gethealth) Damage))
  (if (<= (Variables|Default|Gethealth) 0.0)
    (Development|PrintString "FALL")
    (Game|OpenLevel(byObjectReference) "/Game/Levels/GameOverScreen.GameOverScreen")
    (elif (Variables|Default|GetPlayerHit)
      (Audio|PlaySoundatLocation "/Game/SoundsNMusic/IGSMusicSoundsSomething/FPSCharacterHitSound.FPSCharacterHitSound" (Transformation|GetActorLocation) "0, 0, 0" 1.0 1.0 0.0 0 0 0 0)
      (Utilities|FlowControl|Delay 1.0)
      (Variables|Default|SetPlayerHit false)
      (Development|PrintString (Utilities|String|ToString(Float) (Variables|Default|Gethealth)))
      (Variables|Default|GetBloodHitWidget
        (:then
          (Default|PlayHitAnimation (Variables|Default|GetBloodHitWidget)))
        (:else
          (bind _returnvalue (UserInterface|CreateWidget "/Game/Alex/AlexM/UI/BloodEffect.BloodEffect_C" (Game|GetPlayerController 0)))
          (bind _output_get (Variables|Default|SetBloodHitWidget _returnvalue))
          (UserInterface|Viewport|AddtoViewport _output_get 0)
          (Default|PlayHitAnimation (Variables|Default|GetBloodHitWidget)))))))

(fn ConstructionScript)

(fn FPSHitDetect
  (bind _fpshands (Variables|Default|GetFPSHands))
  (if (not (Variables|Default|GetEnemyIsHit))
    (bind _outhit (Collision|SphereTraceForObjects (Transformation|GetSocketLocation _fpshands "Blade_Start") (Transformation|GetSocketLocation _fpshands "Blade_End") 1e+01 (Utilities|Array|MakeArray "ObjectTypeQuery3") false 0 "None"))
    (Utilities|IsValid (.HitActor (Collision|BreakHitResult _outhit))
      (:Is%20Valid
        (if (Actor|ActorHasTag (.HitActor (Collision|BreakHitResult _outhit)) "Zombie") ; Checks a condition
          (Variables|Default|SetEnemyIsHit true)
          (Game|Damage|ApplyDamage (.HitActor (Collision|BreakHitResult _outhit)) (Variables|Default|GetMacheteDamage) 0 0) ; If the condition is true, then it passes on\nover here and applies damages to the\nZombie.
          (CallFunction|MeleeDamageDelayTaken)
          (Class|AISenseDamage|ReportDamageEvent (.HitActor (Collision|BreakHitResult _outhit)) self 0.0 (Transformation|GetActorLocation) "0, 0, 0" "None") ; This is just a Damage Report
        )))))

(fn SpawnMachetes
  (if (not (Variables|Default|GetMachete_PickedUP))
    (bind _outactors (Actor|GetAllActorsOfClass "/Game/Alex/AlexM/Blueprints/WeaponSpawner_BP.WeaponSpawner_BP_C"))
    (for _array_element _outactors
      (bind _asweapon_spawner_bp (Utilities|Casting|CastToWeaponSpawner_BP _array_element))
      (Default|RandomSpawner _asweapon_spawner_bp))))

(fn DestroyMachetes
  (if (Variables|Default|GetMachete_PickedUP)
    (bind _outactors (Actor|GetAllActorsOfClass "/Game/Alex/AlexM/Blueprints/Assets/Pickup_BP/Machete_PickUp_BP.Machete_PickUp_BP_C"))
    (for _array_element _outactors
      (Actor|DestroyActor _array_element))))