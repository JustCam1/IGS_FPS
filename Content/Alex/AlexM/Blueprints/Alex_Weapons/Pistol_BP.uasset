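; Pistol weapon Blueprint that handles firing feedback and wall-proximity detection for the first-person arms and gun.
; StartShooting calls FireWeapon, then, if PlayAnimation is set, plays the recoil animation, a 2D gunshot sound and the arms' fire montage.
; Every Tick, two concentric sphere traces at the Muzzle socket set WallHit (inner) and OuterTrace (outer) as the basis for anti-clipping.
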(event EventBeginPlay
  (|CallParentFunction) ; This node is disabled and will not be called.\nDrag off pins to build functionality.
)

(event Collision|EventActorBeginOverlap
  (params (OtherActor :type Actor%20Object%20Reference))
  (|CallParentFunction OtherActor) ; This node is disabled and will not be called.\nDrag off pins to build functionality.
)

(event EventTick
  (params (DeltaSeconds :type Float%20%28single-precision%29))
  (bind _weapon (Variables|Default|GetWeapon))
  (bind _weapon_2 (Variables|Default|GetWeapon))
  (bind _returnvalue (Transformation|GetSocketLocation _weapon "Muzzle"))
  (bind _returnvalue_2 (Transformation|GetSocketLocation _weapon_2 "Muzzle"))
  ;[1 1 1] Beginning of Clipping Mechanics for the player arms and gun.
  (bind _returnvalue_3 (Collision|SphereTraceForObjects _returnvalue_2 (+ _returnvalue_2 (* (Math|Vector|GetRightVector _weapon_2) 5.0)) 6.0 (Utilities|Array|MakeArray "ObjectTypeQuery1" "ObjectTypeQuery2" "ObjectTypeQuery4") false 0 "None")) ; Creates a sphere collision out side of the Socket
  (Variables|Default|SetWall_Hit _returnvalue_3) ; Check if it is hitting something
  (bind _returnvalue_4 (Collision|SphereTraceForObjects _returnvalue (+ _returnvalue (* (Math|Vector|GetRightVector _weapon) 5.0)) 1e+01 (Utilities|Array|MakeArray "ObjectTypeQuery1" "ObjectTypeQuery2" "ObjectTypeQuery4") false 0 "None" true "(R=0.088914,G=0.103548,B=1.000000,A=1.000000)")) ; This is a repeat but for the outside Sphere Collision
  (Variables|Default|SetOuter_Trace _returnvalue_4) ; Checks if it is also hitting a wall
)

(event EventStartShooting
  ;[1 1 1] Plays Animation and Sound when the Shooting_IA is called.
  (CallFunction|FireWeapon)
  (if (Variables|Default|GetPlayAnimation?)
    (Components|Animation|PlayAnimation (Variables|Default|GetWeapon) "/Game/Alex/AlexM/Blender_FPS/Pistol/Pistol_Recoil.Pistol_Recoil" false)
    (Audio|PlaySound2D "/Game/Alex/AlexM/Blender_FPS/Pistol/9mm-pistol-shoot-short-reverb-7152.9mm-pistol-shoot-short-reverb-7152" 1.0 1.0 0.0 0 0)
    (Animation|Montage|PlayMontage (Variables|/Game/Alex/AlexM/Blueprints/fpscharacter_bp.fpscharacter_bp_C|GetFPSHands (Variables|Default|GetPlayerRef)) "/Game/Alex/AlexM/Blender_FPS/Pistol/Arm_Pistol_Fire_v2_Montage.Arm_Pistol_Fire_v2_Montage")))

(fn ConstructionScript
  (|CallParentFunction))