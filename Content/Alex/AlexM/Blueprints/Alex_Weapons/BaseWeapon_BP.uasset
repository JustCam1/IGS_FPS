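; Base weapon actor for the FPS player, with empty shooting and swing events and shared logic for guns and melee weapons.
; FireWeapon spends ammo on a camera-forward line trace that damages and reports hits on actors tagged "Zombie".
; Reload refills the magazine from reserve ammo.
; Melee durability drops per call; at zero the weapon destroys itself, calls the player's SpawnMachetes, switches to no weapon and updates player state.
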(event Custom|Start%20Shooting)

(event Custom|Swing)

(event Custom|Stop%20Shooting)

(event Custom|DestroyThisActor
  (Actor|DestroyActor))

(event EventBeginPlay
  (bind _asfpscharacter_bp (Utilities|Casting|CastTofpscharacter_bp (Game|GetPlayerCharacter 0)))
  (Variables|Default|SetFPS_Ref _asfpscharacter_bp))

(event Collision|EventActorBeginOverlap
  (params (OtherActor :type Actor%20Object%20Reference)))

(event EventTick
  (params (DeltaSeconds :type Float%20%28single-precision%29)))

(fn ConstructionScript)

(fn FireWeapon
  (bind _playerref (Variables|Default|GetPlayerRef))
  (bind _camera (Variables|/Game/Alex/AlexM/Blueprints/fpscharacter_bp.fpscharacter_bp_C|GetCamera _playerref))
  (bind _returnvalue (Transformation|GetWorldLocation _camera))
  (if (> (Variables|Default|GetCurrent%20Ammo) 0)
    (Variables|Default|SetPlayAnimation? true)
    (bind _outhit (Collision|LineTraceByChannel _returnvalue (+ _returnvalue (* (Math|Vector|GetForwardVector _camera) 3e+03)) "TraceTypeQuery1" false 0 "ForOneFrame")) ; This is basically a ray cast.
    (Math|Integer|DecrementInt (Variables|Default|GetCurrent%20Ammo)
      (:%20%20
        (Utilities|IsValid (.HitActor (Collision|BreakHitResult _outhit))
          (:Is%20Valid
            (if (Actor|ActorHasTag (.HitActor (Collision|BreakHitResult _outhit)) "Zombie") ; Checks a condition
              (Game|Damage|ApplyDamage (.HitActor (Collision|BreakHitResult _outhit)) (Variables|Default|GetDamage) 0 0) ; If the condition is true, then it passes on\nover here and applies damages to the\nZombie.
              (Class|AISenseDamage|ReportDamageEvent (.HitActor (Collision|BreakHitResult _outhit)) self 0.0 (Transformation|GetActorLocation) "0, 0, 0" "None") ; This is just a Damage Report
            )))))
    (else
      (Variables|Default|SetPlayAnimation? false))))

(fn Reload
  (bind _output_get (LocalVariables|SetAmmoDifference (- (Variables|Default|GetMag) (Variables|Default|GetCurrent%20Ammo))))
  (if (>= (Variables|Default|GetMax%20Ammo) _output_get)
    (Variables|Default|SetCurrent%20Ammo (Variables|Default|GetMag))
    (Variables|Default|SetMax%20Ammo (- (Variables|Default|GetMax%20Ammo) (LocalVariables|GetAmmoDifference)))
    (Components|Animation|PlayAnimation (Variables|Default|GetWeapon) 0 false)
    (else
      (Variables|Default|SetCurrent%20Ammo (+ (Variables|Default|GetCurrent%20Ammo) (Variables|Default|GetMax%20Ammo)))
      (Variables|Default|SetMax%20Ammo 0))))

(fn MeleeDamageTaken
  (bind _playerref (Variables|Default|GetPlayerRef))
  (if (> (Variables|Default|GetMeleeHealth) 0.0)
    (Variables|Default|SetMeleeHealth (- (Variables|Default|GetMeleeHealth) (Variables|Default|GetMeleeDamageTaken)))
    (if (<= (Variables|Default|GetMeleeHealth) 0.0)
      (CallFunction|DestroyThisActor)
      (Default|SpawnMachetes _playerref)
      (ChildActorComponent|SetChildActorClass (Variables|/Game/Alex/AlexM/Blueprints/fpscharacter_bp.fpscharacter_bp_C|GetWeapon_Child_Actor _playerref) (.weapon (Variables|/Game/Alex/AlexM/Blueprints/fpscharacter_bp.fpscharacter_bp_C|GetNoWeapon _playerref)))
      (Widget|RemovefromParent (Variables|/Game/Alex/AlexM/Blueprints/fpscharacter_bp.fpscharacter_bp_C|GetplayerHudRef _playerref))
      (Default|Update _playerref)
      (Variables|/Game/Alex/AlexM/Blueprints/fpscharacter_bp.fpscharacter_bp_C|SetHas_Melee (Variables|Default|GetPlayerRef) false))))