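; RosemaryDoor is an interactable door that stays locked until the player has a fuse lever count of at least three.
; On Interact it reads that count from the player character, then alternately plays and reverses a timeline that yaws the Sphere component up to 90 degrees, with an opening sound each time.
; While locked, it shows a locked-door prompt on the player's UI, then restores the press-E prompt after a short delay.
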(event Collision|EventActorBeginOverlap
  (params (OtherActor :type Actor%20Object%20Reference)))

(event EventTick
  (params (DeltaSeconds :type Float%20%28single-precision%29)))

(event EventInteract
  (bind _asfpscharacter_bp (Utilities|Casting|CastTofpscharacter_bp (Game|GetPlayerCharacter 0)))
  (bind _output_get (Variables|Default|SetAs%20Fpscharacter%20Bp _asfpscharacter_bp))
  (if (>= (Variables|/Game/Alex/AlexM/Blueprints/fpscharacter_bp.fpscharacter_bp_C|GetFuse_Lever_Count _output_get) 3)
    (Utilities|FlowControl|FlipFlop
      (:A
        (Audio|PlaySound2D "/Game/SoundsNMusic/IGSMusicSoundsSomething/DoorOpening.DoorOpening" 1.0 1.0 0.0 0 0)
        (bind _doortimer (Timeline|DoorTimeline Play)
          (:Update
            (Transformation|SetRelativeRotation (Variables|Default|GetSphere) (Math|Rotator|MakeRotator 0.0 0.0 (* _doortimer 9e+01)) false false))))
      (:B
        (Audio|PlaySound2D "/Game/SoundsNMusic/IGSMusicSoundsSomething/DoorOpening.DoorOpening" 1.0 1.0 0.0 0 0)
        (Timeline|DoorTimeline Reverse)))
    (else
      (Default|LockedDoorPrompt (Variables|/Game/Alex/AlexM/Blueprints/fpscharacter_bp.fpscharacter_bp_C|GetInteractive%20UI%20Ref (Variables|Default|GetAs%20Fpscharacter%20Bp)))
      (Utilities|FlowControl|Delay 0.85)
      (Default|Press[E] (Variables|/Game/Alex/AlexM/Blueprints/fpscharacter_bp.fpscharacter_bp_C|GetInteractive%20UI%20Ref (Variables|Default|GetAs%20Fpscharacter%20Bp))))))

(fn ConstructionScript)