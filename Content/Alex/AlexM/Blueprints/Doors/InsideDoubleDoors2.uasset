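; Interactable interior double door that swings two leaves open and closed and reacts to the first-level fuse box event.
; Interact, unless locked, flip-flops a timeline that rotates two pivot spheres in opposite directions, plays a sound and briefly toggles leaf collision.
; With the player's fuse box flag set, the LockDoors overlap closes an open door once or locks a closed one, setting the player's 2DoorLocked flag.
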(event OnComponentBeginOverlap(LockDoors)
  (params (OverlappedComponent :type Primitive%20Component%20Object%20Reference) (OtherActor :type Actor%20Object%20Reference) (OtherComp :type Primitive%20Component%20Object%20Reference) (OtherBodyIndex :type Integer) (bFromSweep :type Boolean) (SweepResult :type Hit%20Result%20Structure%20%28by%20ref%29))
  (bind _as_fpscharacter_bp (Variables|Default|GetAs%20Fpscharacter%20Bp))
  (Development|PrintString "over")
  (if (and (Variables|/Game/Alex/AlexM/Blueprints/fpscharacter_bp.fpscharacter_bp_C|GetFirstLevelFuseBox _as_fpscharacter_bp) (Variables|Default|GetDoorIsOpen))
    (Utilities|FlowControl|DoOnce false
      (:Completed
        (Variables|/Game/Alex/AlexM/Blueprints/fpscharacter_bp.fpscharacter_bp_C|Set2DoorLocked _as_fpscharacter_bp true)
        (Variables|Default|SetDoorIsOpen false)
        (Collision|SetCollisionEnabled (Variables|Default|GetLeftDoor) "NoCollision")
        (Audio|PlaySound2D "/Game/SoundsNMusic/IGSMusicSoundsSomething/DoorOpening.DoorOpening" 1.0 1.0 0.0 0 0)
        (bind _doortimer (Timeline|DoorTimeline Reverse)
          (:Update
            (Transformation|SetRelativeRotation (Variables|Default|GetSphere) (Math|Rotator|MakeRotator 0.0 0.0 (* _doortimer 9e+01)) false false)
            (Transformation|SetRelativeRotation (Variables|Default|GetSphere1) (Math|Rotator|MakeRotator 0.0 0.0 (* _doortimer -9e+01)) false false)
            (Collision|SetCollisionEnabled (Variables|Default|GetLeftDoor) "QueryAndPhysics")))))
    (elif (and (Variables|/Game/Alex/AlexM/Blueprints/fpscharacter_bp.fpscharacter_bp_C|GetFirstLevelFuseBox _as_fpscharacter_bp) (not (Variables|Default|GetDoorIsOpen)))
      (Variables|Default|SetLOCKED true)
      (Variables|/Game/Alex/AlexM/Blueprints/fpscharacter_bp.fpscharacter_bp_C|Set2DoorLocked _as_fpscharacter_bp true))))

(event EventBeginPlay
  (bind _asfpscharacter_bp (Utilities|Casting|CastTofpscharacter_bp (Game|GetPlayerCharacter 0)))
  (Variables|Default|SetAs%20Fpscharacter%20Bp _asfpscharacter_bp))

(event Collision|EventActorBeginOverlap
  (params (OtherActor :type Actor%20Object%20Reference)))

(event EventTick
  (params (DeltaSeconds :type Float%20%28single-precision%29)))

(event EventInteract
  (bind _leftdoor (Variables|Default|GetLeftDoor))
  (if (not (Variables|Default|GetLOCKED))
    (Utilities|FlowControl|FlipFlop
      (:A
        (Variables|Default|SetDoorIsOpen true)
        (Collision|SetCollisionEnabled _leftdoor "NoCollision")
        (Audio|PlaySound2D "/Game/SoundsNMusic/IGSMusicSoundsSomething/DoorOpening.DoorOpening" 1.0 1.0 0.0 0 0)
        (bind _doortimer (Timeline|DoorTimeline Play)
          (:Update
            (Transformation|SetRelativeRotation (Variables|Default|GetSphere) (Math|Rotator|MakeRotator 0.0 0.0 (* _doortimer 9e+01)) false false)
            (Transformation|SetRelativeRotation (Variables|Default|GetSphere1) (Math|Rotator|MakeRotator 0.0 0.0 (* _doortimer -9e+01)) false false)
            (Collision|SetCollisionEnabled (Variables|Default|GetLeftDoor) "QueryAndPhysics"))))
      (:B
        (Variables|Default|SetDoorIsOpen false)
        (Collision|SetCollisionEnabled _leftdoor "NoCollision")
        (Audio|PlaySound2D "/Game/SoundsNMusic/IGSMusicSoundsSomething/DoorOpening.DoorOpening" 1.0 1.0 0.0 0 0)
        (Timeline|DoorTimeline Reverse)))))

(fn ConstructionScript)