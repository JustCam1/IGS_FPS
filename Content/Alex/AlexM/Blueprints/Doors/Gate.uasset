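; Gate door that swings open once the player has pulled enough fuse levers.
; BeginPlay caches the fpscharacter_bp player character, and Tick compares its FuseLeverCount against MaxLeverCount.
; DoorTimeline plays when the count reaches the maximum and reverses otherwise, driving the InsideGate yaw by up to a quarter turn as its DoorTimer track scales the angle.
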(event EventBeginPlay
  (bind _asfpscharacter_bp (Utilities|Casting|CastTofpscharacter_bp (Game|GetPlayerCharacter 0)))
  (Variables|Default|SetAs%20Fpscharacter%20Bp _asfpscharacter_bp))

(event Collision|EventActorBeginOverlap
  (params (OtherActor :type Actor%20Object%20Reference)))

(event EventTick
  (params (DeltaSeconds :type Float%20%28single-precision%29))
  (bind _as_fpscharacter_bp (Variables|Default|GetAs%20Fpscharacter%20Bp))
  (Utilities|IsValid _as_fpscharacter_bp
    (:Is%20Valid
      (if (>= (Variables|/Game/Alex/AlexM/Blueprints/fpscharacter_bp.fpscharacter_bp_C|GetFuse_Lever_Count _as_fpscharacter_bp) (Variables|/Game/Alex/AlexM/Blueprints/fpscharacter_bp.fpscharacter_bp_C|GetMax_Lever_Count _as_fpscharacter_bp))
        (bind _doortimer (Timeline|DoorTimeline Play)
          (:Update
            (Transformation|SetRelativeRotation (Variables|Default|GetInside_Gate) (Math|Rotator|MakeRotator 0.0 0.0 (* _doortimer 9e+01)) false false)))
        (else
          (Timeline|DoorTimeline Reverse))))))

(fn ConstructionScript)