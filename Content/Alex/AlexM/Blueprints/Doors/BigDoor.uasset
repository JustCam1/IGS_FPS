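; BigDoor is a double door that swings open or closed on alternate Interact calls.
; A FlipFlop plays or reverses DoorTimeline, whose track yaws Sphere and Sphere1 in opposite directions, scaled to 90 degrees.
; Each toggle disables collision on LeftDoor and RightDoor, but every timeline update restores it, so it returns during the swing rather than after it.
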(event EventBeginPlay)

(event Collision|EventActorBeginOverlap
  (params (OtherActor :type Actor%20Object%20Reference)))

(event EventTick
  (params (DeltaSeconds :type Float%20%28single-precision%29)))

(event EventInteract
  (bind _leftdoor (Variables|Default|GetLeftDoor))
  (Utilities|FlowControl|FlipFlop
    (:A
      (Development|PrintString "open")
      (Collision|SetCollisionEnabled _leftdoor "NoCollision")
      (bind _doortimer (Timeline|DoorTimeline Play)
        (:Update
          (Transformation|SetRelativeRotation (Variables|Default|GetSphere) (Math|Rotator|MakeRotator 0.0 0.0 (* _doortimer 9e+01)) false false)
          (Transformation|SetRelativeRotation (Variables|Default|GetSphere1) (Math|Rotator|MakeRotator 0.0 0.0 (* _doortimer -9e+01)) false false)
          (Collision|SetCollisionEnabled (Variables|Default|GetLeftDoor) "QueryAndPhysics"))))
    (:B
      (Development|PrintString "Close")
      (Collision|SetCollisionEnabled _leftdoor "NoCollision")
      (Timeline|DoorTimeline Reverse))))

(fn ConstructionScript)