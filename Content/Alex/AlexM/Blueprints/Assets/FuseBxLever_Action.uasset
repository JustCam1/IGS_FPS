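; Fuse box lever actor meant to open when the player interacts, though that logic is currently unwired.
; BeginPlay caches the fpscharacter_bp player and creates the Interact_BP prompt widget.
; Disconnected chains would show or hide the prompt for the player, play fuse box and lever animations once, set Opened and increase the character's FuseLeverCount.
; The Interact event is empty, so none of those chains run.
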(event EventBeginPlay
  (bind _asfpscharacter_bp (Utilities|Casting|CastTofpscharacter_bp (Game|GetPlayerCharacter 0)))
  (Variables|Default|SetFPS_Ref _asfpscharacter_bp)
  (bind _returnvalue (UserInterface|CreateWidget "/Game/Alex/AlexM/UI/Interact_BP.Interact_BP_C"))
  (Variables|Default|SetPress%20E _returnvalue))

(event Collision|EventActorBeginOverlap
  (params (OtherActor :type Actor%20Object%20Reference)))

(event EventTick
  (params (DeltaSeconds :type Float%20%28single-precision%29)))

(event EventInteract)

(fn ConstructionScript)