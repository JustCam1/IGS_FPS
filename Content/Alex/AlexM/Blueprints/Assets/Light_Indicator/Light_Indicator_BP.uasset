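; Indicator actor with left, middle and right lights that shows the player's fuse lever count.
; On BeginPlay it caches the player as fpscharacter_bp.
; Every Tick it switches on that character's FuseLeverCount and applies a Glow material to the matching light for counts one to three.
; Nothing reverts the material, so lights stay lit as the count rises.
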(event EventBeginPlay
  (bind _asfpscharacter_bp (Utilities|Casting|CastTofpscharacter_bp (Game|GetPlayerCharacter 0)))
  (Variables|Default|SetAs%20Fpscharacter%20Bp _asfpscharacter_bp))

(event EventTick
  (params (DeltaSeconds :type Float%20%28single-precision%29))
  (switch int (Variables|/Game/Alex/AlexM/Blueprints/fpscharacter_bp.fpscharacter_bp_C|GetFuse_Lever_Count (Variables|Default|GetAs%20Fpscharacter%20Bp))
    (:1
      (Rendering|Material|SetMaterial (Variables|Default|GetLeftLight) 0 "/Game/Alex/AlexM/Blueprints/Assets/Light_Indicator/Glow.Glow"))
    (:2
      (Rendering|Material|SetMaterial (Variables|Default|GetMiddleLight) 0 "/Game/Alex/AlexM/Blueprints/Assets/Light_Indicator/Glow.Glow"))
    (:3
      (Rendering|Material|SetMaterial (Variables|Default|GetRightLight) 0 "/Game/Alex/AlexM/Blueprints/Assets/Light_Indicator/Glow.Glow"))))

(fn ConstructionScript)