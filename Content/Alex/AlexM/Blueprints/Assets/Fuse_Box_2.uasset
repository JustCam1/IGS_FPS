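; Interactive fuse box with a hinged door and a one-shot lever that feeds the player's fuse lever progress.
; Interact branches on the player character's NameDetected to pick Lever or Door.
; The lever animates with sound, increments FuseLeverCount, sets FirstLevelFuseBox and disables its collision.
; The door alternates opening and closing through a FlipFlop-driven rotation timeline; lever-reset and hum logic are unconnected.
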(event EventBeginPlay)

(event Collision|EventActorBeginOverlap
  (params (OtherActor :type Actor%20Object%20Reference)))

(event EventInteract
  (bind _asfpscharacter_bp (Utilities|Casting|CastTofpscharacter_bp (Game|Player|GetPlayerPawn 0)))
  (bind _output_get (Variables|Default|SetAs%20Fpscharacter%20Bp _asfpscharacter_bp))
  (switch string (Utilities|String|ToString(Name) (Variables|/Game/Alex/AlexM/Blueprints/fpscharacter_bp.fpscharacter_bp_C|GetNameDetected _output_get))
    (:Lever
      (if (not (Variables|Default|GetLeverDown))
        (Components|Animation|PlayAnimation (Variables|Default|GetLever) "/Game/Alex/AlexM/Blueprints/Assets/New_FuseBox/Just_PullDown_Lever_Anim.Just_PullDown_Lever_Anim" false)
        (Audio|PlaySoundatLocation "/Game/SoundsNMusic/IGSMusicSoundsSomething/PullLeverForFuseBox.PullLeverForFuseBox" (Variables|/Script/Engine.SceneComponent|GetRelativeLocation (Variables|Default|GetLever)) "0, 0, 0" 1.0 1.0 0.0 0 0 0 0)
        (Variables|Default|SetLeverDown true)
        (Variables|/Game/Alex/AlexM/Blueprints/fpscharacter_bp.fpscharacter_bp_C|SetFuse_Lever_Count (Variables|Default|GetAs%20Fpscharacter%20Bp) (+ (Variables|/Game/Alex/AlexM/Blueprints/fpscharacter_bp.fpscharacter_bp_C|GetFuse_Lever_Count (Variables|Default|GetAs%20Fpscharacter%20Bp)) (Variables|Default|GetLeverPulled)))
        (Variables|/Game/Alex/AlexM/Blueprints/fpscharacter_bp.fpscharacter_bp_C|SetFirstLevelFuseBox (Variables|Default|GetAs%20Fpscharacter%20Bp) true)
        (Collision|SetCollisionEnabled (Variables|Default|GetLever) "NoCollision")))
    (:Door
      (Utilities|FlowControl|FlipFlop
        (:A
          (Audio|PlaySound2D "/Game/SoundsNMusic/IGSMusicSoundsSomething/OpenFuseBoxDoor.OpenFuseBoxDoor" 1.0 1.0 0.0 0 0)
          (bind _doortimer (Timeline|Timeline PlayFromStart)
            (:Update
              (Transformation|SetRelativeRotation (Variables|Default|GetSphere) (Math|Rotator|MakeRotator 0.0 0.0 (* _doortimer 1.1e+02)) false false))))
        (:B
          (Audio|PlaySound2D "/Game/SoundsNMusic/IGSMusicSoundsSomething/OpenDoorForFuseBox2.OpenDoorForFuseBox2" 1.0 1.0 0.0 0 0)
          (Timeline|Timeline Reverse))))))

(fn ConstructionScript)