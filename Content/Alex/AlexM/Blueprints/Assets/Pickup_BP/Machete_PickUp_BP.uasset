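; Machete pickup that gives the player a melee weapon when interacted with.
; If the player already has melee, it first spawns an actor slightly above itself, tilted at random, carrying the current weapon's melee health values.
; It then copies its own weapon class and health into the player's Machete slot, swaps the weapon child actor, refreshes player state and HUD, enables attacking and destroys itself.
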(event EventBeginPlay
  (|CallParentFunction) ; This node is disabled and will not be called.\nDrag off pins to build functionality.
)

(event Collision|EventActorBeginOverlap
  (params (OtherActor :type Actor%20Object%20Reference))
  (|CallParentFunction OtherActor) ; This node is disabled and will not be called.\nDrag off pins to build functionality.
)

(event EventTick
  (params (DeltaSeconds :type Float%20%28single-precision%29))
  (|CallParentFunction DeltaSeconds) ; This node is disabled and will not be called.\nDrag off pins to build functionality.
)

(event EventInteract
  (bind _returnvalue (Transformation|GetActorTransform))
  (bind _returnvalue_2 (Math|Random|RandomIntegerinRange 10 15))
  (bind _fps_ref (Variables|Default|GetFps%20Ref))
  (bind _fps_ref_2 (Variables|Default|GetFps%20Ref))
  (bind _weapon_struct (Variables|Default|GetWeapon_Struct))
  (bind _weaponref (Variables|/Game/Alex/AlexM/Blueprints/fpscharacter_bp.fpscharacter_bp_C|GetWeaponRef _fps_ref_2))
  (Default|AmmoHolder _fps_ref_2)
  (Variables|/Game/Alex/AlexM/Blueprints/fpscharacter_bp.fpscharacter_bp_C|SetMachete_PickedUP _fps_ref_2 true)
  (if (Variables|/Game/Alex/AlexM/Blueprints/fpscharacter_bp.fpscharacter_bp_C|GetHas_Melee _fps_ref_2)
    (Game|SpawnActorfromClass :Class "Machete_PickUp_BP_C" :SpawnTransform (Math|Transform|MakeTransform (Math|Vector|MakeVector (.x (.location _returnvalue)) (.y (.location _returnvalue)) (+ (.z (.location _returnvalue)) 8.0)) (Math|Rotator|MakeRotator (Math|Conversions|ToFloat(Integer) _returnvalue_2) (Math|Conversions|ToFloat(Integer) _returnvalue_2) 2.0) "1.000000,1.000000,1.000000") :CollisionHandlingOverride "Undefined" :TransformScaleMethod "MultiplyWithRoot" :Weapon_Struct (Utilities|Struct|MakeWeaponStruct "/Game/Alex/AlexM/Blueprints/Alex_Weapons/Machete_BP.Machete_BP_C" 0 0 (Variables|/Game/Alex/AlexM/Blueprints/Alex_Weapons/BaseWeapon_BP.BaseWeapon_BP_C|GetMeleeHealth _weaponref) (Variables|/Game/Alex/AlexM/Blueprints/Alex_Weapons/BaseWeapon_BP.BaseWeapon_BP_C|GetMeleeMaxHealth _weaponref)) :Instigator 0))
  (Variables|/Game/Alex/AlexM/Blueprints/fpscharacter_bp.fpscharacter_bp_C|SetHas_Melee _fps_ref true)
  (Variables|/Game/Alex/AlexM/Blueprints/fpscharacter_bp.fpscharacter_bp_C|SetMachete _fps_ref (Utilities|Struct|MakeWeaponStruct (.weapon _weapon_struct) 0 0 (.meleehealth _weapon_struct) (.meleemaxhealth _weapon_struct)))
  (Widget|RemovefromParent (Variables|/Game/Alex/AlexM/Blueprints/fpscharacter_bp.fpscharacter_bp_C|GetplayerHudRef _fps_ref))
  (ChildActorComponent|SetChildActorClass (Variables|/Game/Alex/AlexM/Blueprints/fpscharacter_bp.fpscharacter_bp_C|GetWeapon_Child_Actor _fps_ref) (.weapon (Variables|/Game/Alex/AlexM/Blueprints/fpscharacter_bp.fpscharacter_bp_C|GetMachete _fps_ref)))
  (Default|Update _fps_ref)
  (Variables|/Game/Alex/AlexM/Blueprints/fpscharacter_bp.fpscharacter_bp_C|SetCanAttack _fps_ref true)
  (Actor|DestroyActor))

(fn ConstructionScript
  (|CallParentFunction))