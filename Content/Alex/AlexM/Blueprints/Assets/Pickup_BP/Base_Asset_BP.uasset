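; Base actor Blueprint for interactable pickups that shows an interact prompt widget when the player comes near.
; On BeginPlay it caches the FPS character reference and creates an Interact_BP widget.
; Sphere overlap adds the prompt to the viewport for the player, while any overlap end removes it.
; Interact is an empty event, and InteractionEnd destroys the actor.
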(event OnComponentBeginOverlap(Sphere)
  (params (OverlappedComponent :type Primitive%20Component%20Object%20Reference) (OtherActor :type Actor%20Object%20Reference) (OtherComp :type Primitive%20Component%20Object%20Reference) (OtherBodyIndex :type Integer) (bFromSweep :type Boolean) (SweepResult :type Hit%20Result%20Structure%20%28by%20ref%29))
  (if (== OtherActor (Game|GetPlayerCharacter 0))
    (UserInterface|Viewport|AddtoViewport (Variables|Default|GetPressE) 0)))

(event OnComponentEndOverlap(Sphere)
  (params (OverlappedComponent :type Primitive%20Component%20Object%20Reference) (OtherActor :type Actor%20Object%20Reference) (OtherComp :type Primitive%20Component%20Object%20Reference) (OtherBodyIndex :type Integer))
  (if true
    (Widget|RemovefromParent (Variables|Default|GetPressE))))

(event Custom|Interaction%20End
  (Actor|DestroyActor))

(event EventBeginPlay
  (bind _asfpscharacter_bp (Utilities|Casting|CastTofpscharacter_bp (Game|GetPlayerCharacter 0)))
  (Variables|Default|SetFPS_Ref _asfpscharacter_bp)
  (bind _returnvalue (UserInterface|CreateWidget "/Game/Alex/AlexM/UI/Interact_BP.Interact_BP_C"))
  (Variables|Default|SetPressE _returnvalue))

(event EventTick
  (params (DeltaSeconds :type Float%20%28single-precision%29)))

(event EventInteract)

(fn ConstructionScript)