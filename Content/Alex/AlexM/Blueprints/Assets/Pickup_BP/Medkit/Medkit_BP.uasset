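; Medkit pickup actor that restores player health when interacted with.
; Interact adds AddHealth to FPSRef's Health only while it is below 100, without clamping the result.
; It then plays the health recovery widget's animation, creating the widget if none is valid.
; Only that creation branch plays the pickup sound and a random voice line, then calls InteractionEnd.
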(event EventBeginPlay
  (|CallParentFunction) ; This node is disabled and will not be called.\nDrag off pins to build functionality.
)

(event Collision|EventActorBeginOverlap
  (params (OtherActor :type Actor%20Object%20Reference))
  (|CallParentFunction OtherActor) ; This node is disabled and will not be called.\nDrag off pins to build functionality.
)

(event EventTick
  (params (DeltaSeconds :type Float%20%28single-precision%29))
  (|CallParentFunction DeltaSeconds) ; This node is disabled and will not be called.\nDrag off pins to build functionality.
)

(event EventInteract
  (bind _fps_ref (Variables|Default|GetFPS_Ref))
  (if (not (>= (Variables|/Game/Alex/AlexM/Blueprints/fpscharacter_bp.fpscharacter_bp_C|Gethealth _fps_ref) 1e+02))
    (Variables|/Game/Alex/AlexM/Blueprints/fpscharacter_bp.fpscharacter_bp_C|Sethealth _fps_ref (+ (Variables|Default|GetAddHealth) (Variables|/Game/Alex/AlexM/Blueprints/fpscharacter_bp.fpscharacter_bp_C|Gethealth _fps_ref)))
    (Variables|Default|GetHealthRecoveryWidget
      (:then
        (Default|PlayHitAnimation (Variables|Default|GetHealthRecoveryWidget)))
      (:else
        (bind _returnvalue (UserInterface|CreateWidget "/Game/Alex/AlexM/UI/HealthEffect.HealthEffect_C" (Game|GetPlayerController 0)))
        (bind _output_get (Variables|Default|SetHealthRecoveryWidget _returnvalue))
        (UserInterface|Viewport|AddtoViewport _output_get 0)
        (Default|PlayHitAnimation (Variables|Default|GetHealthRecoveryWidget))
        (Audio|PlaySound2D "/Engine/VREditor/Sounds/UI/Enter_Play.Enter_Play" 1.0 1.0 0.0 0 0)
        (Audio|PlaySound2D (Utilities|Select :Index (Math|Random|RandomIntegerinRange 0 3) :Option%200 "/Game/SoundsNMusic/IGSMusicSoundsSomething/VLs/healthPickUpLine1.healthPickUpLine1" :Option%201 "/Game/SoundsNMusic/IGSMusicSoundsSomething/VLs/HealthPickupLine2.HealthPickupLine2" :Option%202 "/Game/SoundsNMusic/IGSMusicSoundsSomething/VLs/HealthPickupLine3.HealthPickupLine3") 1.0 1.0 0.0 0 0)
        (CallFunction|InteractionEnd)))))

(fn ConstructionScript
  (|CallParentFunction))