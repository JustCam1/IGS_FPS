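; Overhead light actor that stays dark until the player character's fuse lever count reaches its maximum.
; BeginPlay caches the player's fpscharacter_bp and hides the rect lights, then Tick polls the lever count and keeps them hidden while it falls short.
; On reaching the maximum, a DoOnce shows the lights with a flicker light function material, swapping to a stop-flicker material after a short delay.
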(event EventBeginPlay
  (bind _asfpscharacter_bp (Utilities|Casting|CastTofpscharacter_bp (Game|GetPlayerCharacter 0)))
  (Variables|Default|SetAs%20Fpscharacter%20Bp _asfpscharacter_bp)
  (Rendering|SetVisibility (Variables|Default|GetRect_Lights) false false))

(event Collision|EventActorBeginOverlap
  (params (OtherActor :type Actor%20Object%20Reference)))

(event EventTick
  (params (DeltaSeconds :type Float%20%28single-precision%29))
  (bind _as_fpscharacter_bp (Variables|Default|GetAs%20Fpscharacter%20Bp))
  (bind _rect_lights (Variables|Default|GetRect_Lights))
  (if (>= (Variables|/Game/Alex/AlexM/Blueprints/fpscharacter_bp.fpscharacter_bp_C|GetFuse_Lever_Count _as_fpscharacter_bp) (Variables|/Game/Alex/AlexM/Blueprints/fpscharacter_bp.fpscharacter_bp_C|GetMax_Lever_Count _as_fpscharacter_bp))
    (Utilities|FlowControl|DoOnce false
      (:Completed
        (Rendering|Components|Light|SetLightFunctionMaterial (Variables|Default|GetRect_Lights) "/Game/Alex/AlexM/Blender_FPS/OverheadLights/Flicker_1P5sec_M.Flicker_1P5sec_M")
        (Rendering|SetVisibility _rect_lights true false)
        (Utilities|FlowControl|Delay 1.0)
        (Rendering|Components|Light|SetLightFunctionMaterial (Variables|Default|GetRect_Lights) "/Game/Alex/AlexM/Blender_FPS/OverheadLights/Stop_Flicker_M.Stop_Flicker_M")))
    (else
      (Rendering|SetVisibility _rect_lights false false))))

(fn ConstructionScript)