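; Base zombie-girl enemy that chases the player, strikes with melee attacks and reacts to being shot.
; ChasePlayer re-issues a move and attack every three seconds, with a delayed right-hand sphere trace applying damage.
; Damage reduces health, plays random hit reactions and switches AIC_EnemyBase to attacking; lethal damage plays a random death montage before destroying the actor.
; Helper functions expose patrol route, ideal range and speed presets.
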(event OnComponentHit(CapsuleComponent)
  (params (HitComponent :type Primitive%20Component%20Object%20Reference) (OtherActor :type Actor%20Object%20Reference) (OtherComp :type Primitive%20Component%20Object%20Reference) (NormalImpulse :type Vector :default "0, 0, 0") (Hit :type Hit%20Result%20Structure%20%28by%20ref%29)))

(event OnComponentHit(Mesh)
  (params (HitComponent :type Primitive%20Component%20Object%20Reference) (OtherActor :type Actor%20Object%20Reference) (OtherComp :type Primitive%20Component%20Object%20Reference) (NormalImpulse :type Vector :default "0, 0, 0") (Hit :type Hit%20Result%20Structure%20%28by%20ref%29)))

(event Custom|ChasePlayer
  (if (Variables|Default|GetisDead)
    (Actor|DestroyActor)
    (else
      (AI|AIMoveTo self "0, 0, 0" (Game|GetPlayerCharacter 0) 5e+01 false
        (:then
          (CallFunction|Attack)
          (Utilities|FlowControl|Delay 3.0)
          (CallFunction|ChasePlayer))))))

(event Custom|Attack
  (Animation|Montage|PlayMontage (Variables|Character|GetMesh) "/Game/ZombieAnimations/Scratch_Zombie__female/Zombie_Attack_Montage.Zombie_Attack_Montage"
    (:then
      (Utilities|FlowControl|Delay 0.5)
      (Audio|PlaySoundatLocation "/Game/SoundsNMusic/IGSMusicSoundsSomething/GirlZombieAttackSound.GirlZombieAttackSound" (Transformation|GetActorLocation) "0, 0, 0" 1.0 1.0 0.0 0 0 0 0)
      (CallFunction|HitDection))
    (:OnCompleted
      (Default|CallAttackonEnd :!label _label))
    (:OnInterrupted
      (goto _label))))

(event Custom|Play%20Death
  (Variables|Default|SetisDead true)
  (Utilities|FlowControl|DoOnce false
    (:Completed
      (Collision|SetCollisionEnabled (Variables|Character|GetMesh) "NoCollision")
      (Components|Activation|Deactivate (Variables|Character|GetCharacterMovement))
      (Animation|Montage|PlayMontage (Variables|Character|GetMesh) (Utilities|Select :Index (Math|Random|RandomIntegerinRange 0 3) :Option%200 "/Game/Alex/Alex_Animations/Zombie_Animations/Zombie_Girl/Death/Death_From_Right_Montage.Death_From_Right_Montage" :Option%201 "/Game/Alex/Alex_Animations/Zombie_Animations/Zombie_Girl/Death/Flying_Back_Death_Montage.Flying_Back_Death_Montage" :Option%202 "/Game/Alex/Alex_Animations/Zombie_Animations/Zombie_Girl/Death/Standing_Death_Left_01_Montage.Standing_Death_Left_01_Montage" :Option%203 "/Game/Alex/Alex_Animations/Zombie_Animations/Zombie_Girl/Death/Standing_React_Death_Backward_Montage.Standing_React_Death_Backward_Montage")
        (:then
          (Audio|PlaySoundatLocation 0 (Transformation|GetActorLocation) "0, 0, 0" 1.0 1.0 0.0 0 0 0 0))
        (:OnBlendOut
          (Variables|Default|SetisDead true)
          (Components|Movement|StopMovementImmediately (Variables|Character|GetCharacterMovement))
          (Actor|DestroyActor))))))

(event EventBeginPlay
  (Variables|Default|SetisDead false))

(event Game|Damage|EventAnyDamage
  (params (Damage :type Float%20%28single-precision%29) (DamageType :type Damage%20Type%20Object%20Reference) (InstigatedBy :type Controller%20Object%20Reference) (DamageCauser :type Actor%20Object%20Reference))
  (bind _returnvalue (Pawn|GetController))
  (Variables|Default|SetDamage Damage)
  (if (> (Variables|Default|GetHealth) 0.0)
    (if (not (Variables|Default|GetGettingHit))
      (Variables|Default|SetGettingHit true)
      (bind _output_get (Variables|Default|SetHealth (- (Variables|Default|GetHealth) (Variables|Default|GetDamage))))
      (if (<= _output_get 0.0)
        (CallFunction|PlayDeath)
        (else
          (Components|Activation|Deactivate (Variables|Character|GetCharacterMovement))
          (Animation|Montage|PlayMontage (Variables|Character|GetMesh) (Utilities|Select :Index (Math|Random|RandomIntegerinRange 0 2) :Option%200 "/Game/Alex/Alex_Animations/Zombie_Animations/Zombie_Girl/Hit_Effect/Head_Hit_Montage.Head_Hit_Montage" :Option%201 "/Game/Alex/Alex_Animations/Zombie_Animations/Zombie_Girl/Hit_Effect/Hit_To_Body_Montage.Hit_To_Body_Montage" :Option%202 "/Game/Alex/Alex_Animations/Zombie_Animations/Zombie_Girl/Hit_Effect/Zombie_Reaction_Hit_Montage.Zombie_Reaction_Hit_Montage" :Option%203 0) 1.5
            (:then
              (Audio|PlaySoundatLocation "/Game/SoundsNMusic/IGSMusicSoundsSomething/ShotSoundZombieGirl.ShotSoundZombieGirl" (Transformation|GetActorLocation) "0, 0, 0" 1.0 1.0 0.0 0 0 0 0))
            (:OnCompleted
              (Components|Activation|Activate (Variables|Character|GetCharacterMovement) false :!label _label))
            (:OnBlendOut
              (goto _label)))
          (bind _asaic_enemy_base (Utilities|Casting|CastToAIC_EnemyBase _returnvalue))
          (bind _output_get_2 (Variables|Default|SetAIC_Ref _asaic_enemy_base))
          (Default|SetStateasAttacking _output_get_2 _returnvalue)
          (Utilities|FlowControl|Delay 0.5)
          (Variables|Default|SetGettingHit false))))))

(fn ConstructionScript)

(fn HitDection
  (bind _mesh (Variables|Character|GetMesh))
  (bind _returnvalue (Transformation|GetSocketLocation _mesh "RightHand"))
  (bind _outhit (Collision|SphereTraceForObjects _returnvalue _returnvalue 5e+01 (Utilities|Array|MakeArray "ObjectTypeQuery3") false 0 "ForDuration"))
  (bind _asfpscharacter_bp (Utilities|Casting|CastTofpscharacter_bp (.HitActor (Collision|BreakHitResult _outhit))))
  (Game|Damage|ApplyDamage _asfpscharacter_bp 0.5 0 0)
  (bind _asbp_rosemary (Utilities|Casting|CastToBP_Rosemary (.HitActor (Collision|BreakHitResult _outhit))))
  (Game|Damage|ApplyDamage _asbp_rosemary 0.5 0 0))

(fn GetIdealRange
  (return 0.0 0.0))

(fn GetPatrolRoute
  (return (Variables|AI|GetPatrolRoutes)))

(fn SetMovementSpeed
  (params (Speed :type E_MovementSpeed%20Enum :default "NewEnumerator0"))
  (bind _output_get (Variables|/Script/Engine.CharacterMovementComponent|SetMaxWalkSpeed (Variables|Character|GetCharacterMovement) (Utilities|Select :Index Speed :NewEnumerator0 0.0 :NewEnumerator1 5e+01 :NewEnumerator2 1e+02 :NewEnumerator3 2e+02)))
  (return _output_get))