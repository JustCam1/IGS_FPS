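; Spitting zombie enemy that screams, turns and spawns projectiles when it sees a pawn, and destroys itself when health runs out.
; Pawn sensing alternates Rosemary and FPS-character casts via FlipFlop, but both aim at and directly damage the FPS-character reference, with a cooldown.
; Capsule hits deal delayed contact damage.
; Helper functions expose combat ranges, patrol route and speed tiers; ChasePlayer is never called here.
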(event OnComponentHit(CapsuleComponent)
  (params (HitComponent :type Primitive%20Component%20Object%20Reference) (OtherActor :type Actor%20Object%20Reference) (OtherComp :type Primitive%20Component%20Object%20Reference) (NormalImpulse :type Vector :default "0, 0, 0") (Hit :type Hit%20Result%20Structure%20%28by%20ref%29))
  (bind _asfpscharacter_bp (Utilities|Casting|CastTofpscharacter_bp OtherActor))
  (Utilities|FlowControl|Delay 0.7)
  (Game|Damage|ApplyDamage _asfpscharacter_bp 2e+01 0 0)
  (bind _asbp_rosemary (Utilities|Casting|CastToBP_Rosemary OtherActor))
  (Utilities|FlowControl|Delay 0.7)
  (Game|Damage|ApplyDamage _asbp_rosemary 2e+01 0 0))

(event OnSeePawn(PawnSensing)
  (params (Pawn :type Pawn%20Object%20Reference))
  (Animation|Montage|PlayMontage (Variables|Character|GetMesh) "/Game/ZombieAnimations/SpitZOmbie/Zombie_Scream_Montage.Zombie_Scream_Montage"
    (:then
      (Utilities|FlowControl|FlipFlop
        (:A
          (bind _asbp_rosemary (Utilities|Casting|CastToBP_Rosemary Pawn)))
        (:B
          (bind _asfpscharacter_bp (Utilities|Casting|CastTofpscharacter_bp Pawn))))
      (Transformation|SetActorRotation (Math|Rotator|FindRelativeLookatRotation (Math|Conversions|ToTransform(Vector) (Transformation|GetActorLocation)) (Transformation|GetActorLocation _asfpscharacter_bp)))
      (if (Variables|Default|GetcanAttack)
        (Game|SpawnActorfromClass "/Game/FirstPerson/Blueprints/BP_FirstPersonProjectile.BP_FirstPersonProjectile_C" (Transformation|GetWorldTransform (Variables|Default|GetSpawnLocationProjectile)) "Undefined" "MultiplyWithRoot" 0 0)
        (Game|Damage|ApplyDamage _asfpscharacter_bp 5.0 0 0)
        (Variables|Default|SetcanAttack false)
        (Utilities|FlowControl|Delay 1.0)
        (Variables|Default|SetcanAttack true)))))

(event OnComponentHit(Mesh)
  (params (HitComponent :type Primitive%20Component%20Object%20Reference) (OtherActor :type Actor%20Object%20Reference) (OtherComp :type Primitive%20Component%20Object%20Reference) (NormalImpulse :type Vector :default "0, 0, 0") (Hit :type Hit%20Result%20Structure%20%28by%20ref%29)))

(event Custom|ChasePlayer
  (AI|AIMoveTo self "0, 0, 0" (Game|GetPlayerCharacter 0) 5e+01 false))

(event Custom|Attack
  (Animation|Montage|PlayMontage (Variables|Character|GetMesh) "/Game/ZombieAnimations/SpitZOmbie/Zombie_Scream_Montage.Zombie_Scream_Montage"
    (:OnCompleted
      _)
    (:OnInterrupted
      _))
  (Default|CallAttackonEnd))

(event EventBeginPlay)

(event Game|Damage|EventAnyDamage
  (params (Damage :type Float%20%28single-precision%29) (DamageType :type Damage%20Type%20Object%20Reference) (InstigatedBy :type Controller%20Object%20Reference) (DamageCauser :type Actor%20Object%20Reference))
  (bind _output_get (Variables|Default|SetHealth (- (Variables|Default|GetHealth) Damage)))
  (if (<= _output_get 0.0)
    (Utilities|FlowControl|DoOnce false
      (:Completed
        (Variables|Default|SetisDead true)
        (Components|Movement|StopMovementImmediately (Variables|Character|GetCharacterMovement))
        (Actor|DestroyActor)))))

(fn ConstructionScript)

(fn GetIdealRange
  (return 1.5e+02 3.5e+02))

(fn GetPatrolRoute
  (return (Variables|AI|GetPatrolRoutes)))

(fn SetMovementSpeed
  (params (Speed :type E_MovementSpeed%20Enum :default "NewEnumerator0"))
  (bind _output_get (Variables|/Script/Engine.CharacterMovementComponent|SetMaxWalkSpeed (Variables|Character|GetCharacterMovement) (Utilities|Select :Index Speed :NewEnumerator0 0.0 :NewEnumerator1 5e+01 :NewEnumerator2 1e+02 :NewEnumerator3 2e+02)))
  (return _output_get))