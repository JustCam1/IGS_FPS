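; Base enemy Blueprint, apparently a zombie, with player chasing, a montage attack and a patrol route getter.
; ChasePlayer issues an AI move toward the player, attacks immediately without waiting for arrival, then repeats itself after a delay.
; Attack calls CallAttackOnEnd when the montage completes or is interrupted.
; BeginPlay is empty, so nothing here starts the chase; GetPatrolRoute only returns PatrolRoutes.
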(event Custom|ChasePlayer
  (AI|AIMoveTo self "0, 0, 0" (Game|GetPlayerCharacter 0) 5e+01 false
    (:then
      (CallFunction|Attack)
      (Utilities|FlowControl|Delay 3.0)
      (CallFunction|ChasePlayer))))

(event Custom|Attack
  (Animation|Montage|PlayMontage (Variables|Character|GetMesh) "/Game/ZombieAnimations/Scratch_Zombie__female/Zombie_Attack_Montage.Zombie_Attack_Montage"
    (:OnCompleted
      _)
    (:OnInterrupted
      _))
  (Default|CallAttackonEnd))

(event EventBeginPlay)

(fn ConstructionScript)

(fn GetPatrolRoute
  (return (Variables|AI|GetPatrolRoutes)))